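; Player character Blueprint that handles weapon switching and right-mouse aiming.
; Keys 1 and 2 replace the held gun with the primary or secondary class, or destroy it if none is set.
; New guns get ammo from SZInventory, attach to weapon_r, enable controller-yaw rotation and refresh the HUD from SZGunDataComp.
; Aiming slows walking, resets crosshair spread and drives camera boom length through a Timeline, reversed on release.
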(event EventBeginPlay
  (if (not (Utilities|Map|Contains (Variables|Default|GetAmmoMap) "NewEnumerator0"))
    (Variables|Default|SetAmmoMap (Variables|Default|GetAmmoMap))))

(event Custom|StartCameraAiming
  ;[0.15 0.15 0.15 0.5] 카메라 세팅
  (CallFunction|SetMaxWalkSpeed 2.5e+02)
  (bind _value (Timeline|Timeline Play)
    (:Update
      (Variables|/Script/Engine.SpringArmComponent|SetTargetArmLength (Variables|Default|GetCameraBoom) (* _value 2e+02)))))

(event Custom|StopCameraAiming
  ;[0.15 0.15 0.15 0.5] 카메라 세팅
  (CallFunction|SetMaxWalkSpeed 5e+02)
  (bind _value (Timeline|Timeline Reverse)
    (:Update
      (Variables|/Script/Engine.SpringArmComponent|SetTargetArmLength (Variables|Default|GetCameraBoom) (* _value 2e+02)))))

(event Custom|SetMaxWalkSpeed
  (params (Max%20Walk%20Speed :type Float%20%28single-precision%29))
  ;[0.15 0.15 0.15 0.5] 걷기 속도
  (Variables|/Script/Engine.CharacterMovementComponent|SetMaxWalkSpeed (Variables|Character|GetCharacterMovement) Max%20Walk%20Speed)
  (Default|TryResetSpread (Variables|Default|GetCT_Cmpt_Crosshair)))

(event Input|KeyboardEvents|1
  (params (Key :type Key%20Structure))
  (bind _bp_skm_primarygun (Variables|Default|GetBP_SKM_PrimaryGun))
  ;[0.15 0.15 0.15 0.5] 번호별 무기 세팅
  (:Pressed
    (if (Utilities|IsValidClass _bp_skm_primarygun)
      (CallFunction|CreateWeapon _bp_skm_primarygun)
      (else
        (Class|SZCharacterPlayer|DestroyWeapon)))))

(event Input|MouseEvents|RightMouseButton
  (params (Key :type Key%20Structure))
  ;[0.15 0.15 0.15 0.5] 확대 줌
  (:Pressed
    (CallFunction|StartCameraAiming))
  (:Released
    (CallFunction|StopCameraAiming)))

(event Input|KeyboardEvents|2
  (params (Key :type Key%20Structure))
  (bind _bp_skm_secondarygun (Variables|Default|GetBP_SKM_SecondaryGun))
  ;[0.15 0.15 0.15 0.5] 번호별 무기 세팅
  (:Pressed
    (if (Utilities|IsValidClass _bp_skm_secondarygun)
      (CallFunction|CreateWeapon _bp_skm_secondarygun)
      (else
        (Class|SZCharacterPlayer|DestroyWeapon)))))

(fn ConstructionScript)

(fn CreateWeapon
  (params (class :type Actor%20Class%20Reference))
  (Class|SZCharacterPlayer|DestroyWeapon)
  (bind _returnvalue (Game|SpawnActorfromClass class (Math|Transform|MakeTransform "0, 0, 0" "0, 0, 0" "1.000000,1.000000,1.000000") "Undefined" "MultiplyWithRoot" self 0))
  (bind _output_get (Variables|Default|SetWeaponGun _returnvalue))
  (bind _returnvalue_2 (Class|SZInventoryBaseComponent|SetAmmo (Variables|Default|GetSZInventory) _output_get (Variables|Default|GetGunID)))
  (Utilities|IsValid _returnvalue_2
    (:Is%20Valid
      (bind _output_get_2 (Variables|Default|SetWeaponGun _returnvalue_2))
      (Transformation|AttachComponentToComponent _output_get_2 (Variables|Character|GetMesh) "weapon_r" "SnapToTarget" "SnapToTarget" "SnapToTarget" true)
      (Actor|SetOwner 0)
      (Variables|Default|SetOwnerCharacter 0)
      (CallFunction|UpdateAmmoHUD)
      (Variables|Default|SetbUseControllerRotationYaw true)
      (Variables|/Script/Engine.CharacterMovementComponent|SetbOrientRotationToMovement (Variables|Character|GetCharacterMovement) false))))

(fn UpdateAmmoHUD
  (bind _weapongun (Variables|Default|GetWeaponGun))
  (bind _returnvalue (Actor|GetComponentbyClass _weapongun "/Script/ProjectSeoulZ.SZGunDataComp"))
  (Utilities|IsValid (Variables|Default|GetAmmoWidgetRef)
    (:Is%20Valid
      (Utilities|IsValid _weapongun
        (:Is%20Valid
          (Utilities|IsValid _returnvalue
            (:Is%20Valid
              (Default|SetAmmo (Variables|Default|GetAmmoWidgetRef) (Variables|/Script/ProjectSeoulZ.SZGunDataComp|GetCurrentAmmo _returnvalue) (Variables|/Script/ProjectSeoulZ.SZGunDataComp|GetInventoryAmmo _returnvalue)))))))))