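; BP_Inventory controls a spring-arm camera for the inventory display, driven directly by mouse input.
; Holding the left button enables horizontal rotation, with MouseX yawing the arm, and the right button resets its transform and length.
; The wheel zooms within a clamped arm length; wheel-up's large step snaps straight to the closest distance, while wheel-down backs out gradually.
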(event Input|MouseEvents|MouseX
  (params (AxisValue :type Float%20%28single-precision%29))
  ;[0.15 0.15 0.15 0.5] 회전
  ;;[0.15 0.15 0.15 0.5] 가로 회전
  (if (Variables|Default|GetSetRotate)
    (Transformation|SetRelativeRotation (Variables|Default|GetSpringArm) (Math|Rotator|CombineRotators (Transformation|GetWorldRotation (Variables|Default|GetSpringArm)) (Math|Rotator|MakeRotator 0.0 0.0 (* AxisValue -4.0))) false false)))

(event Input|MouseEvents|LeftMouseButton
  (params (Key :type Key%20Structure :default "None"))
  ;[0.15 0.15 0.15 0.5] 회전
  ;;[0.15 0.15 0.15 0.5] Allows Rotation
  (:Pressed
    (Variables|Default|SetSetRotate true))
  (:Released
    (Variables|Default|SetSetRotate false)))

(event Input|MouseEvents|RightMouseButton
  (params (Key :type Key%20Structure :default "None"))
  ;[0.15 0.15 0.15 0.5] Reset Display
  (:Pressed
    (Transformation|SetRelativeLocationAndRotation (Variables|Default|GetSpringArm) "0.000000,0.000000,120.000000" "-5.000000,-180.000000,0.000000" false false)
    (Variables|/Script/Engine.SpringArmComponent|SetTargetArmLength (Variables|Default|GetSpringArm) 1.6e+02)))

(event Input|MouseEvents|MouseWheelUp
  (params (Key :type Key%20Structure :default "None"))
  (bind _springarm (Variables|Default|GetSpringArm))
  ;[0.15 0.15 0.15 0.5] Zoom In & Out
  (:Pressed
    (Variables|/Script/Engine.SpringArmComponent|SetTargetArmLength _springarm (Math|Float|Clamp(Float) (- (Variables|/Script/Engine.SpringArmComponent|GetTargetArmLength _springarm) 2e+02) 1e+02 1.8e+02))))

(event Input|MouseEvents|MouseWheelDown
  (params (Key :type Key%20Structure :default "None"))
  (bind _springarm (Variables|Default|GetSpringArm))
  ;[0.15 0.15 0.15 0.5] Zoom In & Out
  (:Pressed
    (Variables|/Script/Engine.SpringArmComponent|SetTargetArmLength _springarm (Math|Float|Clamp(Float) (+ (Variables|/Script/Engine.SpringArmComponent|GetTargetArmLength _springarm) 2e+01) 1e+02 1.8e+02))))

(fn ConstructionScript)