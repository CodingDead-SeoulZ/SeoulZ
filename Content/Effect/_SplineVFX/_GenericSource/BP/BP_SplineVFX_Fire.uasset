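; Pooled fire spline VFX actor that animates a Niagara effect's growth over time.
; On BeginPlay it stores its box, Niagara and start components as Hit, NiagaraEffect and ReferencePoint.
; Each spawn from the pool restarts a timeline that writes its value to the Niagara User.Progress parameter and the Progress variable.
; The construction script sets the timeline's play rate from GrowSpeed.
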(event EventBeginPlay
  (Variables|Default|SetHit (Variables|Default|GetBox))
  (Variables|Default|SetNiagaraEffect (Variables|Default|GetNiagara))
  (Variables|Default|SetReferencePoint (Variables|Default|GetStart)))

(event Collision|EventActorBeginOverlap
  (params (OtherActor :type Actor%20Object%20Reference)))

(event EventTick
  (params (DeltaSeconds :type Float%20%28single-precision%29)))

(event EventOnSpawnfromPoolBlueprint
  (bind _newtrack_0 (Timeline|Timeline PlayFromStart)
    (:Update
      (Niagara|SetNiagaraVariable(Float) (Variables|Default|GetNiagara) "User.Progress" _newtrack_0)
      (Variables|Default|SetProgress _newtrack_0))))

(fn ConstructionScript
  (Components|Timeline|SetPlayRate (Variables|Default|GetTimeline) (Variables|Default|GetGrowSpeed)))